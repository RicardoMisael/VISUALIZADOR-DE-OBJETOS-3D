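; BP_Cuchillo is a knife actor that spins in place and toggles its look on key press.
; On BeginPlay it enables input from the first player controller.
; Pressing E prints a debug message and uses a FlipFlop to alternate the static mesh between two knife materials.
; Tick rotates it around local yaw at a constant, frame-rate independent speed.
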(event EventTick
  (params (DeltaSeconds :type Float%20%28single-precision%29))
  (Transformation|AddActorLocalRotation (Math|Rotator|MakeRotator 0.0 0.0 (* (Utilities|Time|GetWorldDeltaSeconds) 45.0)) false false))

(event EventBeginPlay
  (Input|EnableInput (Game|GetPlayerController 0)))

(event Input|KeyboardEvents|E
  (params (Key :type Key%20Structure :default "None"))
  (:Pressed
    (Development|PrintString "Presione E" true true "(R=0.000000,G=0.660000,B=1.000000,A=1.000000)" 15.0)
    (Utilities|FlowControl|FlipFlop
      (:A
        (Rendering|Material|SetMaterial (Variables|Default|GetStaticMesh) 0 (Variables|Default|GetMaterialCuchillo)))
      (:B
        (Rendering|Material|SetMaterial (Variables|Default|GetStaticMesh) 0 (Variables|Default|GetMaterialCuchillo2))))))

(fn ConstructionScript)